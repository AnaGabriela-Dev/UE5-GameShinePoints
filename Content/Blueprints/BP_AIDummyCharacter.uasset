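; AI dummy character with an overhead health bar widget that shows and turns toward the camera while the player is near.
; DetectionSphere overlaps with BP_PlayerCharacter show the widget and start a looping timer, presumably driving the look-at rotation update, instead of using Tick.
; Leaving the sphere hides the widget and clears the timer.
; BeginPlay leaves the widget visible, so it displays unrotated until an overlap changes it.
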(event `UpdateHealthBarRotation`
  ; Update Rotation
  (`SceneComponent.K2_SetWorldRotation` (`self.EnemyHealthWidget`) (`KismetMathLibrary.FindLookAtRotation` (`SceneComponent.K2_GetComponentLocation` (`self.EnemyHealthWidget`)) (`PlayerCameraManager.GetCameraLocation` (`GameplayStatics.GetPlayerCameraManager` 0))) false false))

(event `self.ReceiveBeginPlay`
  ; BeginPlay
  (`SceneComponent.SetHiddenInGame` (`self.EnemyHealthWidget`) false false))

(event `self.DetectionSphere.OnComponentBeginOverlap`
  (params (OverlappedComponent :type "PrimitiveComponent Object Reference") (OtherActor :type "Actor Object Reference") (OtherComp :type "PrimitiveComponent Object Reference") (OtherBodyIndex :type Integer) (bFromSweep :type Boolean) (SweepResult :type "HitResult Structure (by ref)"))
  ; LifeBar Visibility Logic
  (cast `/Game/Blueprints/BP_PlayerCharacter` OtherActor)
  (`SceneComponent.SetHiddenInGame` (`self.EnemyHealthWidget`) false false)
  (bind _returnvalue (`KismetSystemLibrary.K2_SetTimerDelegate` (`|CreateDelegate` :!event `UpdateHealthBarRotation`) 0.05 true))
  (set `self.TimerHandle` _returnvalue))

(event `self.DetectionSphere.OnComponentEndOverlap`
  (params (OverlappedComponent :type "PrimitiveComponent Object Reference") (OtherActor :type "Actor Object Reference") (OtherComp :type "PrimitiveComponent Object Reference") (OtherBodyIndex :type Integer))
  ; LifeBar Visibility Logic
  (cast `/Game/Blueprints/BP_PlayerCharacter` OtherActor)
  (`SceneComponent.SetHiddenInGame` (`self.EnemyHealthWidget`) true false)
  (`KismetSystemLibrary.K2_ClearAndInvalidateTimerHandle` (`self.TimerHandle`)))

(fn `UserConstructionScript`)