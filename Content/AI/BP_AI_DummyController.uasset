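; AI controller for a dummy AI that runs BT_Dummy and feeds it sight and hearing perception through the Blackboard.
; Sight of the player sets TargetActor; losing sight clears it and stores the player's position as LastKnownLocation.
; Hearing writes the stimulus position to TargetLocation only while no valid TargetActor exists, so sight takes priority over sound.
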(event `self.ReceiveBeginPlay`
  (`self.RunBehaviorTree` "/Game/AI/BT_Dummy.BT_Dummy"))

(event `self.AIPerception.OnTargetPerceptionUpdated`
  (params (Actor :type "Actor Object Reference") (Stimulus :type "AIStimulus Structure"))
  (`self.HandleSightSense` Actor Stimulus)
  (`self.HandleSoundSense` Stimulus))

(fn `HandleSightSense`
  (params (Actor :type "Actor Object Reference") (Stimulus :type "AIStimulus Structure"))
  (bind (_stimulus_age _stimulus_expirationage _stimulus_strength _stimulus_stimuluslocation _stimulus_receiverlocation _stimulus_tag _stimulus_bsuccessfullysensed) (break `AIStimulus` (`local.Stimulus`)))
  (bind _returnvalue (`AIPerceptionSystem.GetSenseClassForStimulus` Stimulus))
  (if (== _returnvalue "/Script/AIModule.AISense_Sight")
    (if (== (`local.Actor`) (`GameplayStatics.GetPlayerCharacter` 0))
      (`BlackboardComponent.SetValueAsObject` (`self.Blackboard`) "TargetActor" (`KismetMathLibrary.SelectObject` (`GameplayStatics.GetPlayerCharacter` 0) null _stimulus_bsuccessfullysensed))
      (if (not _stimulus_bsuccessfullysensed)
        (`BlackboardComponent.SetValueAsVector` (`self.Blackboard`) "LastKnownLocation" (`self.K2_GetActorLocation` (`GameplayStatics.GetPlayerCharacter` 0))))
      (else
        (return)))
    (else
      (return))))

(fn `HandleSoundSense`
  (params (Stimulus :type "AIStimulus Structure (by ref)"))
  (bind _returnvalue (`AIPerceptionSystem.GetSenseClassForStimulus` Stimulus))
  (if (== _returnvalue "/Script/AIModule.AISense_Hearing")
    (if (!= (`self.Instigator`) self)
      (`/Engine/EditorBlueprintResources/StandardMacros.IsValid` (`BlackboardComponent.GetValueAsObject` (`self.Blackboard`) "TargetActor")
        (:`Is Not Valid`
          (`BlackboardComponent.SetValueAsVector` (`self.Blackboard`) "TargetLocation" (`.StimulusLocation` (break `AIStimulus` (`local.Stimulus`)))))))))

(fn `UserConstructionScript`)